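; BP_OpenPath is a maze path switch that swaps which of two walls, left or right, blocks the way.
; Each OpenPath event waits through a short Delay, then a FlipFlop alternates between the two states.
; The active wall becomes visible with full collision while the other is hidden with collision disabled, and a debug string is printed.
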(event `self.ReceiveBeginPlay`)

(event `self.ReceiveActorBeginOverlap`
  (params (OtherActor :type "Actor Object Reference")))

(event `self.ReceiveTick`
  (params (DeltaSeconds :type "Float (single-precision)")))

(event `OpenPath`
  (bind _pathwall_r (`self.PathWall-R`))
  (bind _pathwall_l (`self.PathWall-L`))
  (`KismetSystemLibrary.Delay` 1.0)
  (`/Engine/EditorBlueprintResources/StandardMacros.FlipFlop`
    (:`A`
      (`SceneComponent.SetVisibility` _pathwall_l true false)
      (`SceneComponent.SetVisibility` _pathwall_r false false)
      (`PrimitiveComponent.SetCollisionEnabled` _pathwall_l "QueryAndPhysics")
      (`PrimitiveComponent.SetCollisionEnabled` _pathwall_r "NoCollision")
      (`KismetSystemLibrary.PrintString` "A visble"))
    (:`B`
      (`SceneComponent.SetVisibility` _pathwall_r true false)
      (`SceneComponent.SetVisibility` _pathwall_l false false)
      (`PrimitiveComponent.SetCollisionEnabled` _pathwall_r "QueryAndPhysics")
      (`PrimitiveComponent.SetCollisionEnabled` _pathwall_l "NoCollision")
      (`KismetSystemLibrary.PrintString` "b visble"))))

(fn `UserConstructionScript`)