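; End_Antorch reveals torch lights in the maze game to match the player's TotalAllStart count.
; BeginPlay caches the player's BP_UserBall, then every Tick loops the Antorch array and shows the Light at index count minus one.
; Nothing hides a Light again, so revealed ones stay on.
; The duplicate Visibility function is never called, and the construction script's mesh and material assignment is disconnected.
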(event `self.ReceiveBeginPlay`
  (bind _asbp_user_ball (cast `/Game/Maze_Game/Blueprints/BP_UserBall` (`GameplayStatics.GetPlayerPawn` 0)))
  (set `self.User Ball` _asbp_user_ball))

(event `self.ReceiveTick`
  (params (DeltaSeconds :type "Float (single-precision)"))
  ;[1 1 1] Starts
  (for (_array_element _array_index) (`self.Antorch`)
    (if (== _array_index (- (`/Game/Maze_Game/Blueprints/BP_UserBall.TotalAllStart` (`self.User Ball`)) 1))
      (`SceneComponent.SetVisibility` (`/Game/Maze_Game/Blueprints/End_Antorch.Light` _array_element) true false))))

(fn `UserConstructionScript`)

(fn `Visibility`
  (for (_array_element _array_index) (`self.Antorch`)
    (if (== _array_index (- (`/Game/Maze_Game/Blueprints/BP_UserBall.TotalAllStart` (`self.User Ball`)) 1))
      (`SceneComponent.SetVisibility` (`/Game/Maze_Game/Blueprints/End_Antorch.Light` _array_element) true false))))