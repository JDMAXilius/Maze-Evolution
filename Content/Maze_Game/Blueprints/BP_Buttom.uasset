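; BP_Buttom is a pressure button in the maze game that triggers linked gates when the player ball overlaps its Box.
; Any overlap plays a sound, but only BP_UserBall sets Push and, one second later, calls TrigerGate on GateAray.
; When the ball leaves, the PBotum particle component, templated in the construction script, is destroyed after a delay.
; BeginPlay calls MaterialBottum, which is empty because its SetMaterial node is disconnected.
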(event `self.ReceiveBeginPlay`
  (`self.MaterialBottum` (`self.Buttom`)))

(event `self.ReceiveActorBeginOverlap`
  (params (OtherActor :type "Actor Object Reference")))

(event `self.ReceiveTick`
  (params (DeltaSeconds :type "Float (single-precision)")))

(event `self.Box.OnComponentBeginOverlap`
  (params (OtherActor :type "Actor Object Reference") (OtherComp :type "PrimitiveComponent Object Reference") (OtherBodyIndex :type Integer) (bFromSweep :type Boolean) (SweepResult :type "HitResult Structure (by ref)"))
  (`GameplayStatics.PlaySound2D` "/Game/Maze_Game/Sound/Take/Enemy_Summon_Appear01_Cue.Enemy_Summon_Appear01_Cue")
  (cast `/Game/Maze_Game/Blueprints/BP_UserBall` OtherActor)
  (set `self.push` true)
  (`KismetSystemLibrary.Delay` 1.0)
  (`/Game/Maze_Game/Blueprints/BP_Gate.triger gate` (`self.gate aray`)))

(event `self.Box.OnComponentEndOverlap`
  (params (OtherActor :type "Actor Object Reference") (OtherComp :type "PrimitiveComponent Object Reference") (OtherBodyIndex :type Integer))
  (cast `/Game/Maze_Game/Blueprints/BP_UserBall` OtherActor)
  (`KismetSystemLibrary.Delay` 1.0)
  (`ActorComponent.K2_DestroyComponent` (`self.P_Botum`)))

(fn `MaterialBottum`)

(fn `UserConstructionScript`
  (`ParticleSystemComponent.SetTemplate` (`self.P_Botum`) (`self.Particule`)))