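; BP_Start is a pickup actor in the maze game that rewards the player ball when touched.
; On StaticMesh2 overlap it plays a pickup cue, then casts the other actor to BP_UserBall, calls AddStart, adds XP and calls its XP function.
; A pixel-bomb emitter spawns at the actor, is deactivated after a short delay, and the pickup destroys itself.
; The sound plays before the cast, so any overlapping actor triggers it.
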(event `self.StaticMesh2.OnComponentBeginOverlap`
  (params (OverlappedComponent :type "PrimitiveComponent Object Reference") (OtherActor :type "Actor Object Reference") (OtherComp :type "PrimitiveComponent Object Reference") (OtherBodyIndex :type Integer) (bFromSweep :type Boolean) (SweepResult :type "HitResult Structure (by ref)"))
  (`GameplayStatics.PlaySound2D` "/Game/Maze_Game/Sound/Take/Key_Pickup02_Cue.Key_Pickup02_Cue" 1.0 1.0 0.0 null null)
  (bind _asbp_user_ball (cast `/Game/Maze_Game/Blueprints/BP_UserBall` OtherActor))
  (`/Game/Maze_Game/Blueprints/BP_UserBall.AddStart` _asbp_user_ball)
  (set `/Game/Maze_Game/Blueprints/BP_UserBall.CurrentXP` (+ (`/Game/Maze_Game/Blueprints/BP_UserBall.CurrentXP` _asbp_user_ball) 200) _asbp_user_ball)
  (`/Game/Maze_Game/Blueprints/BP_UserBall.XP` _asbp_user_ball)
  (bind _returnvalue (`GameplayStatics.SpawnEmitterAtLocation` "/Game/Maze_Game/Particles/P_PixelBomb.P_PixelBomb" (`self.K2_GetActorLocation`) (struct) (1.0 1.0 1.0) false))
  (`KismetSystemLibrary.Delay` 0.1)
  (`ActorComponent.Deactivate` _returnvalue)
  (`self.K2_DestroyActor`))

(fn `UserConstructionScript`)