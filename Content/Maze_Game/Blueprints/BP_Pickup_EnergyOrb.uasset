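; BP_Pickup_EnergyOrb is a collectible energy orb that rewards the player's BP_UserBall.
; Overlapping its Interior component plays a sound before the cast, so any overlapping actor triggers the audio.
; For the ball, it adds an orb, points and XP, then shows an animated floating Points_Text widget.
; A pixel-bomb particle bursts at the ball and is deactivated after a brief delay before the orb destroys itself.
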(event `self.Interior.OnComponentBeginOverlap`
  (params (OtherActor :type "Actor Object Reference") (OtherComp :type "PrimitiveComponent Object Reference") (OtherBodyIndex :type Integer) (bFromSweep :type Boolean) (SweepResult :type "HitResult Structure (by ref)"))
  (`GameplayStatics.PlaySound2D` "/Game/Maze_Game/Sound/Take/UI_XPGreenNumber01_Cue.UI_XPGreenNumber01_Cue")
  (bind _asbp_user_ball (cast `/Game/Maze_Game/Blueprints/BP_UserBall` OtherActor))
  (`/Game/Maze_Game/Blueprints/BP_UserBall.AddEnergyOrb` _asbp_user_ball)
  (`/Game/Maze_Game/Blueprints/BP_UserBall.AddPoints` _asbp_user_ball)
  (`/Game/Maze_Game/Blueprints/BP_UserBall.XP` _asbp_user_ball)
  (bind _returnvalue (`|CreateWidget` "/Game/Maze_Game/UI/Points_Text.Points_Text_C" null self))
  (`UserWidget.AddToViewport` _returnvalue 0)
  (`UserWidget.PlayAnimation` _returnvalue (`/Game/Maze_Game/UI/Points_Text.Floating Text` _returnvalue) 0.0 1 "Forward")
  (set `/Game/Maze_Game/UI/Points_Text.Float Text` 10 _returnvalue)
  (bind _returnvalue_2 (`GameplayStatics.SpawnEmitterAtLocation` "/Game/Maze_Game/Particles/P_PixelBomb.P_PixelBomb" (`SceneComponent.K2_GetComponentLocation` (`/Game/Maze_Game/Blueprints/BP_UserBall.Ball` _asbp_user_ball))))
  (`KismetSystemLibrary.Delay` 0.1)
  (`ActorComponent.Deactivate` _returnvalue_2)
  (`self.K2_DestroyActor`))

(fn `UserConstructionScript`
  (`parent.UserConstructionScript`))