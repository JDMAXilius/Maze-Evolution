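; BP_ButtomPath is a maze button that opens a path when the player's BP_UserBall rolls onto it.
; Its Box overlap calls OpenPath on a referenced object and swaps the Base mesh to a pushed material, restoring the default material when the ball leaves.
; The summon sound plays for any overlapping actor, since it fires before the ball cast.
; The construction script applies the default material.
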(event `self.ReceiveActorBeginOverlap`
  (params (OtherActor :type "Actor Object Reference")))

(event `self.ReceiveTick`
  (params (DeltaSeconds :type "Float (single-precision)")))

(event `self.Box.OnComponentBeginOverlap`
  (params (OtherActor :type "Actor Object Reference") (OtherComp :type "PrimitiveComponent Object Reference") (OtherBodyIndex :type Integer) (bFromSweep :type Boolean) (SweepResult :type "HitResult Structure (by ref)"))
  (`GameplayStatics.PlaySound2D` "/Game/Maze_Game/Sound/Take/Enemy_Summon_Appear01_Cue.Enemy_Summon_Appear01_Cue")
  (cast `/Game/Maze_Game/Blueprints/BP_UserBall` OtherActor)
  (`/Game/Maze_Game/Blueprints/BP_OpenPath.OpenPath` (`self.OpenPath`))
  (`PrimitiveComponent.SetMaterial` (`self.Base`) 0 (`self.Material_Push`)))

(event `self.Box.OnComponentEndOverlap`
  (params (OtherActor :type "Actor Object Reference") (OtherComp :type "PrimitiveComponent Object Reference") (OtherBodyIndex :type Integer))
  (cast `/Game/Maze_Game/Blueprints/BP_UserBall` OtherActor)
  (`PrimitiveComponent.SetMaterial` (`self.Base`) 0 (`self.Material`)))

(fn `UserConstructionScript`
  (`PrimitiveComponent.SetMaterial` (`self.Base`) 0 (`self.Material`)))